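; Clock actor for the Lv_1 minigame that tracks time of day and displays it through a Lv_1_Die widget created on BeginPlay.
; A looping timer runs IncrementTime, which either copies the system clock or advances Time by TimeStep with 24-hour wrap, depending on UserRealWorldTime.
; Each tick of that timer pushes time and date to the widget.
; UpdateSun is called but empty, and its sun-rotation logic is disconnected.
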(event EventBeginPlay
  (bind _returnvalue (UserInterface|CreateWidget "/Game/_MiniGame/Lv_1/Lv_1_Die.Lv_1_Die_C"))
  (bind _output_get (Variables|Default|SetWPDie _returnvalue))
  (Variables|/Game/_MiniGame/Lv_1/Lv_1_Die.Lv_1_Die_C|SetUserRealWorldTime _output_get false)
  (Utilities|Time|SetTimerbyFunctionName 0 "IncrementTime" (Math|Float|SelectFloat 1.0 0.1 (Variables|Default|GetUserRealWorldTime)) true))

(event Collision|EventActorBeginOverlap
  (params (OtherActor :type Actor%20Object%20Reference)))

(event EventTick
  (params (DeltaSeconds :type Float%20%28single-precision%29)))

(fn ConstructionScript
  (CallFunction|UpdateSun))

(fn IncrementTime
  (bind _returnvalue (Math|DateTime|Now))
  (bind (_year _month _day _hour _minute) (Math|DateTime|BreakDateTime _returnvalue))
  (if (Variables|Default|GetUserRealWorldTime)
    (Variables|Default|SetTime (+ (Math|Conversions|ToFloat(Integer) _hour) (/ _minute 60)))
    (Variables|Default|SetYear _year)
    (Variables|Default|SetMonth _month)
    (Variables|Default|SetDay _day)
    (else
      (Variables|Default|SetTime (Math|Float|%(Float) (+ (Variables|Default|GetTime) (Variables|Default|GetTimeStep)) 24.0))))
  (CallFunction|UpdateSun)
  (bind _wpdie (Variables|Default|GetWPDie)
    (:then
      (Default|SetTimeText _wpdie (Math|Float|Floor (Variables|Default|GetTime)) (Math|Float|Truncate (* (- (Variables|Default|GetTime) (Math|Float|Floor (Variables|Default|GetTime))) 6e+01)) (Variables|Default|GetYear) (Variables|Default|GetMonth) (Variables|Default|GetDay)))
    (:else)))

(fn UpdateSun)