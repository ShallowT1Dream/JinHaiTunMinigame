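; BP_Button is a minigame trigger that spawns balls and ends play when one reaches it.
; A self-rearming timer, randomized to a few seconds, spawns a 球 at a random point around each 球生成点 entry and passes it a reference to the button.
; A ball overlapping the Box is destroyed, adds the death widget from BPDie once, and switches input to UI-only with the cursor shown.
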(event OnComponentBeginOverlap(Box)
  (params (OverlappedComponent :type Primitive%20Component%20Object%20Reference) (OtherActor :type Actor%20Object%20Reference) (OtherComp :type Primitive%20Component%20Object%20Reference) (OtherBodyIndex :type Integer) (bFromSweep :type Boolean) (SweepResult :type Hit%20Result%20Structure%20%28by%20ref%29))
  (bind _returnvalue (Game|GetPlayerController 0))
  (bind _as球 (Utilities|Casting|CastTo球 OtherActor))
  (Development|PrintString "碰到了按钮")
  (Actor|DestroyActor _as球)
  (Utilities|FlowControl|Sequence
    (:then_0
      (Utilities|FlowControl|DoOnce false
        (:Completed
          (UserInterface|Viewport|AddtoViewport (Variables|/Game/_MiniGame/Lv_1/BP_Die.BP_Die_C|GetWPDie (Variables|Default|GetBP_Die)) 0))))
    (:then_1
      (Input|SetInputModeUIOnly _returnvalue 0 "LockInFullscreen" false)
      (Variables|/Script/Engine.PlayerController|SetbShowMouseCursor _returnvalue true))))

(event Custom|刷球
  (for _array_element (Variables|Default|Get球生成点)
    (bind _returnvalue (Game|SpawnActorfromClass "/Game/_MiniGame/Lv_1/球.球_C" (Math|Conversions|ToTransform(Vector) (Math|Random|RandomPointinBoundingBox (Transformation|GetWorldLocation (Variables|/Game/_MiniGame/Lv_1/生成球的点.生成球的点_C|GetSphere _array_element)) "500.000000,500.000000,500.000000")) "Undefined" "MultiplyWithRoot" 0 0))
    (Variables|/Game/_MiniGame/Lv_1/球.球_C|SetButton _returnvalue self)
    (Utilities|Time|SetTimerbyEvent (delegate Custom|刷球) (Math|Random|RandomFloatinRange 3.0 5.0))))

(event EventBeginPlay
  (Utilities|Time|SetTimerbyEvent (delegate Custom|刷球) (Math|Random|RandomFloatinRange 3.0 5.0)))

(event Collision|EventActorBeginOverlap
  (params (OtherActor :type Actor%20Object%20Reference)))

(event EventTick
  (params (DeltaSeconds :type Float%20%28single-precision%29)))

(event EventInteract)

(fn ConstructionScript)