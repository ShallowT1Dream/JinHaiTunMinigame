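; BP_Button is an interactable button that counts presses toward a required total, apparently meant to open a list of linked doors.
; Each Interact increments and prints the counter, then plays a timeline that lerps the Sphere's relative height downward.
; Once the threshold is reached it loops over DoorsToOpen, but the loop body is empty: the OpenDoor call is disconnected, so no door opens.
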(event EventBeginPlay
  (Variables|Default|SetCurrentPresses 0))

(event Collision|EventActorBeginOverlap
  (params (OtherActor :type Actor%20Object%20Reference)))

(event EventTick
  (params (DeltaSeconds :type Float%20%28single-precision%29)))

(event EventInteract
  (Utilities|FlowControl|Sequence
    (:then_0
      (Variables|Default|SetCurrentPresses (+ (Variables|Default|GetCurrentPresses) 1))
      (Development|PrintString (Utilities|String|ToString(Integer) (Variables|Default|GetCurrentPresses)))
      (if (>= (Variables|Default|GetCurrentPresses) (Variables|Default|GetPressesRequired))
        (for _array_element (Variables|Default|GetDoorsToOpen)
          _)))
    (:then_1
      (bind _buttonopen (Timeline|时间轴 Play)
        (:Update
          (Transformation|SetRelativeLocation (Variables|Default|GetSphere) (Math|Vector|MakeVector 0.0 0.0 (Math|Float|Lerp 3e+01 0.0 _buttonopen)) false false))))))

(fn ConstructionScript)